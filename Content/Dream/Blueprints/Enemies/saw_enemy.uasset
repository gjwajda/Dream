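; Saw enemy hazard that travels between two placed points and hurts the player hero on contact.
; On BeginPlay it snaps to PointA, waits a short random delay, then plays a timeline that lerps its location toward PointB without sweeping.
; A sphere overlap casts to AlienHero_BP and applies fixed damage through the hero's DamageSystem.
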(event OnComponentBeginOverlap(Sphere)
  (params (OtherActor :type Actor%20Object%20Reference) (OtherComp :type Primitive%20Component%20Object%20Reference) (OtherBodyIndex :type Integer) (bFromSweep :type Boolean) (SweepResult :type Hit%20Result%20Structure%20%28by%20ref%29))
  ;[1 1 1] Enemy Damage
  (bind _asalien_hero_bp (Utilities|Casting|CastToAlienHero_BP OtherActor))
  (Default|DamageSystem _asalien_hero_bp 0.5))

(event EventBeginPlay
  (bind _point_a (Variables|Default|GetPoint-A))
  (bind _returnvalue (Transformation|GetActorLocation _point_a))
  ;[1 1 1] Enemy Movement
  (Transformation|SetActorLocation _returnvalue false)
  (Utilities|FlowControl|Delay (Math|Random|RandomFloatinRange 0.0 2.0))
  (bind _alphavalue (Timeline|Timeline_0 Play)
    (:Update
      (Transformation|SetActorLocation (Math|Vector|Lerp(Vector) _returnvalue (Transformation|GetActorLocation (Variables|Default|GetPoint-B)) _alphavalue) false))))

(event Collision|EventActorBeginOverlap
  (params (OtherActor :type Actor%20Object%20Reference)))

(event EventTick
  (params (DeltaSeconds :type Float%20%28single-precision%29)))

(fn ConstructionScript)