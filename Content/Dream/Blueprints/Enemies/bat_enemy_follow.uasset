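; Paper2D bat enemy that chases the player while the hero is inside its Trigger, then flies back to its start and hangs.
; Tick flips the sprite toward the player and drives MoveComponentTo on the flipbook.
; Sphere overlap damages AlienHero and briefly disables JSphere so it cannot be killed.
; A JSphere hit otherwise kills it, playing a death flipbook and timeline rotation before destruction.
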(event OnComponentBeginOverlap(Sphere)
  (params (OtherActor :type Actor%20Object%20Reference) (OtherComp :type Primitive%20Component%20Object%20Reference) (OtherBodyIndex :type Integer) (bFromSweep :type Boolean) (SweepResult :type Hit%20Result%20Structure%20%28by%20ref%29))
  (bind _jsphere (Variables|Default|GetJSphere))
  ;[1 1 1] Enemy Damage + Animation
  (bind _asalien_hero_bp (Utilities|Casting|CastToAlienHero_BP OtherActor))
  (Variables|Default|SetHitFirst true)
  (Default|DamageSystem _asalien_hero_bp 0.5)
  (Collision|SetCollisionEnabled _jsphere "NoCollision")
  (Variables|Default|SetnoHit true)
  (Utilities|FlowControl|Delay 2.8)
  (Variables|Default|SetHitFirst false)
  (Collision|SetCollisionEnabled _jsphere "QueryAndPhysics")
  (Variables|Default|SetnoHit false))

(event OnComponentHit(JSphere)
  (params (OtherActor :type Actor%20Object%20Reference) (OtherComp :type Primitive%20Component%20Object%20Reference) (NormalImpulse :type Vector :default "0, 0, 0") (Hit :type Hit%20Result%20Structure%20%28by%20ref%29))
  ;[1 1 1] Enemy Damage + Animation
  (if (not (Variables|Default|GetnoHit))
    (if (not (Variables|Default|GetHitFirst))
      (Variables|Default|SetDead true)
      (Components|DestroyComponent (Variables|Default|GetSphere))
      (Components|DestroyComponent (Variables|Default|GetJSphere))
      (Sprite|SetFlipbook (Variables|Default|GetPaperFlipbook) "/Game/Dream/Sprites/Enemies/Frames/bat_dead.bat_dead")
      (bind (_direction _rotation_yaw _rotation_roll) (Timeline|Fly%20Timeline Play)
        (:Update
          (Transformation|SetActorRotation (Math|Rotator|MakeRotator 0.0 _rotation_yaw _rotation_roll))
          (Utilities|FlowControl|Delay 3.0)
          (Actor|DestroyActor))))))

(event OnActorBeginOverlap(Trigger)
  (params (OtherActor :type Actor%20Object%20Reference))
  ;[1 1 1] Enemy Movement
  ;;[1 1 1] Follow Check
  (Utilities|Casting|CastToAlienHero_BP OtherActor)
  (Variables|Default|SetFollow true))

(event OnActorEndOverlap(Trigger)
  (params (OtherActor :type Actor%20Object%20Reference))
  (bind _paperflipbook (Variables|Default|GetPaperFlipbook))
  ;[1 1 1] Enemy Movement
  ;;[1 1 1] Follow Check
  (Utilities|Casting|CastToAlienHero_BP OtherActor)
  (Variables|Default|SetFollow false)
  ;;[1 1 1] UnFollow Sequence
  (Utilities|FlowControl|Sequence
    (:then_0
      ;;[1 1 1] Follow Sequence
      (Components|MoveComponentTo _paperflipbook (Variables|Default|GetPlayerLocation) "0, 0, 0" true false 8.0) ; enters at Stop
    )
    (:then_1
      (Components|MoveComponentTo _paperflipbook (Variables|Default|GetOriginalLocation) "0, 0, 0" false false 1.0)
      (Sprite|SetFlipbook _paperflipbook "/Game/Dream/Sprites/Enemies/Frames/bat_hang.bat_hang"))))

(event Custom|Stop%20All
  (bind _paperflipbook (Variables|Default|GetPaperFlipbook))
  ;[1 1 1] Enemy Movement
  (Utilities|FlowControl|Sequence
    (:then_0
      ;;[1 1 1] Follow Sequence
      (Components|MoveComponentTo _paperflipbook (Variables|Default|GetPlayerLocation) "0, 0, 0" true false 8.0) ; enters at Stop
    )
    (:then_1
      ;;[1 1 1] UnFollow Sequence
      (Components|MoveComponentTo _paperflipbook (Variables|Default|GetOriginalLocation) "0, 0, 0" false false 1.0) ; enters at Stop
    )))

(event EventBeginPlay
  ;[1 1 1] Set Location
  (Variables|Default|SetOriginalLocation (Transformation|GetActorLocation)))

(event EventTick
  (params (DeltaSeconds :type Float%20%28single-precision%29))
  (bind _paperflipbook (Variables|Default|GetPaperFlipbook))
  (bind _paperflipbook_2 (Variables|Default|GetPaperFlipbook))
  ;[1 1 1] Enemy Movement
  (Variables|Default|SetPlayerLocation (Transformation|GetActorLocation (Game|GetPlayerCharacter 0)))
  (Variables|Default|SetBatLocation (Transformation|GetActorLocation))
  (if (>= (.x (Class|KismetMathLibrary|GetDirectionVector (Variables|Default|GetBatLocation) (Variables|Default|GetPlayerLocation))) 0.0)
    (Transformation|SetWorldScale3D _paperflipbook_2 "-1.000000,1.000000,1.000000")
    (else
      (Transformation|SetWorldScale3D _paperflipbook_2 "1.000000,1.000000,1.000000")))
  (if (Variables|Default|GetDead)
    (CallFunction|StopAll)
    (elif (Variables|Default|GetFollow)
      ;;[1 1 1] Follow Sequence
      (Utilities|FlowControl|Sequence
        (:then_0
          ;;[1 1 1] UnFollow Sequence
          (Components|MoveComponentTo _paperflipbook (Variables|Default|GetOriginalLocation) "0, 0, 0" false false 1.0) ; enters at Stop
        )
        (:then_1
          (Sprite|SetFlipbook _paperflipbook "/Game/Dream/Sprites/Enemies/bat_animation.bat_animation")
          (Components|MoveComponentTo _paperflipbook (Variables|Default|GetPlayerLocation) "0, 0, 0" true false 8.0))))))

(event Collision|EventActorBeginOverlap
  (params (OtherActor :type Actor%20Object%20Reference)))

(fn ConstructionScript)