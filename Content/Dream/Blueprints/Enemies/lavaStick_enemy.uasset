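; Lava stick (snake) enemy that damages the AlienHero on contact and can be killed by a hit on its sphere collider.
; Box overlap with the hero deals damage and briefly sets HitFirst, which blocks sphere hits from killing it.
; An unblocked sphere hit from any actor removes both colliders, swaps to the death flipbook, rotates the actor via timeline and destroys it after a delay.
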(event OnComponentHit(J_Sphere)
  (params (OtherActor :type Actor%20Object%20Reference) (OtherComp :type Primitive%20Component%20Object%20Reference) (NormalImpulse :type Vector :default "0, 0, 0") (Hit :type Hit%20Result%20Structure%20%28by%20ref%29))
  ;[1 1 1] Enemy Damage + Animation
  (if (not (Variables|Default|GetHitFirst))
    (Components|DestroyComponent (Variables|Default|GetJ_Sphere))
    (Components|DestroyComponent (Variables|Default|GetBox))
    (Sprite|SetFlipbook (Variables|Default|GetPaperFlipbook) "/Game/Dream/Sprites/Enemies/Frames/snakeLava_dead.snakeLava_dead")
    (bind (_direction _rotation_yaw _rotation_roll) (Timeline|Timeline_0 Play)
      (:Update
        (Transformation|SetActorRotation (Math|Rotator|MakeRotator 0.0 _rotation_yaw _rotation_roll))
        (Utilities|FlowControl|Delay 3.0)
        (Actor|DestroyActor)))))

(event OnComponentBeginOverlap(Box)
  (params (OtherActor :type Actor%20Object%20Reference) (OtherComp :type Primitive%20Component%20Object%20Reference) (OtherBodyIndex :type Integer) (bFromSweep :type Boolean) (SweepResult :type Hit%20Result%20Structure%20%28by%20ref%29))
  ;[1 1 1] Enemy Damage + Animation
  (bind _asalien_hero_bp (Utilities|Casting|CastToAlienHero_BP OtherActor))
  (Variables|Default|SetHitFirst true)
  (Default|DamageSystem _asalien_hero_bp 0.5)
  (Utilities|FlowControl|Delay 2.8)
  (Variables|Default|SetHitFirst false))

(event EventBeginPlay)

(event EventTick
  (params (DeltaSeconds :type Float%20%28single-precision%29)))

(fn ConstructionScript)