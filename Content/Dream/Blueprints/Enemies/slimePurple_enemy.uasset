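; Purple slime enemy with a Paper2D flipbook that patrols between two points and damages the AlienHero on overlap.
; A timeline lerps it from PointA toward PointB after a random start delay, mirroring the sprite at the endpoints.
; A hit on the jump sphere kills it unless it recently damaged the hero.
; Death stops movement, removes collision spheres, swaps to the dead flipbook and rotates the actor before destroying it.
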(event OnComponentBeginOverlap(Sphere)
  (params (OtherActor :type Actor%20Object%20Reference) (OtherComp :type Primitive%20Component%20Object%20Reference) (OtherBodyIndex :type Integer) (bFromSweep :type Boolean) (SweepResult :type Hit%20Result%20Structure%20%28by%20ref%29))
  ;[1 1 1] Enemy Damage + Animation
  (bind _asalien_hero_bp (Utilities|Casting|CastToAlienHero_BP OtherActor))
  (Variables|Default|SetHitFirst true)
  (Default|DamageSystem _asalien_hero_bp 0.5)
  (Utilities|FlowControl|Delay 2.8)
  (Variables|Default|SetHitFirst false))

(event OnComponentHit(Jump_Sphere)
  (params (OtherActor :type Actor%20Object%20Reference) (OtherComp :type Primitive%20Component%20Object%20Reference) (NormalImpulse :type Vector :default "0, 0, 0") (Hit :type Hit%20Result%20Structure%20%28by%20ref%29))
  ;[1 1 1] Enemy Damage + Animation
  (if (not (Variables|Default|GetHitFirst))
    (Variables|Default|SetDead true)
    (Components|DestroyComponent (Variables|Default|GetSphere))
    (Components|DestroyComponent (Variables|Default|GetJump_Sphere))
    (Sprite|SetFlipbook (Variables|Default|GetPaperFlipbook) "/Game/Dream/Sprites/Enemies/Frames/slimePurple_dead.slimePurple_dead")
    (bind (_direction _rotation_yaw _rotation_roll) (Timeline|Mouse%20Timeline Play)
      (:Update
        (Transformation|SetActorRotation (Math|Rotator|MakeRotator 0.0 _rotation_yaw _rotation_roll))
        (Utilities|FlowControl|Delay 3.0)
        (Actor|DestroyActor)))))

(event Collision|EventActorBeginOverlap
  (params (OtherActor :type Actor%20Object%20Reference)))

(event EventTick
  (params (DeltaSeconds :type Float%20%28single-precision%29))
  (bind _paperflipbook (Variables|Default|GetPaperFlipbook))
  ;[1 1 1] Check if Dead
  (if (Variables|Default|GetDead)
    ;[1 1 1] Enemy Movement
    (bind _alphavalue (Timeline|Timeline_0 Stop)
      (:Update
        (Transformation|SetActorLocation (Math|Vector|Lerp(Vector) (Transformation|GetActorLocation (Variables|Default|GetPoint-A)) (Transformation|GetActorLocation (Variables|Default|GetPoint-B)) _alphavalue) false)
        (if (>= _alphavalue 0.99)
          (Transformation|SetWorldScale3D _paperflipbook "1.000000,1.000000,1.000000")
          (elif (<= _alphavalue 0.01)
            (Transformation|SetWorldScale3D _paperflipbook "-1.000000,1.000000,1.000000")))))))

(event EventBeginPlay
  (bind _point_a (Variables|Default|GetPoint-A))
  (bind _paperflipbook (Variables|Default|GetPaperFlipbook))
  (bind _returnvalue (Transformation|GetActorLocation _point_a))
  ;[1 1 1] Enemy Movement
  (Transformation|SetActorLocation _returnvalue false)
  (Utilities|FlowControl|Delay (Math|Random|RandomFloatinRange 0.0 2.0))
  (bind _alphavalue (Timeline|Timeline_0 Play)
    (:Update
      (Transformation|SetActorLocation (Math|Vector|Lerp(Vector) _returnvalue (Transformation|GetActorLocation (Variables|Default|GetPoint-B)) _alphavalue) false)
      (if (>= _alphavalue 0.99)
        (Transformation|SetWorldScale3D _paperflipbook "1.000000,1.000000,1.000000")
        (elif (<= _alphavalue 0.01)
          (Transformation|SetWorldScale3D _paperflipbook "-1.000000,1.000000,1.000000"))))))

(fn ConstructionScript)