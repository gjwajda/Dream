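; MyHUD is a HUD Blueprint that shows a loading screen and opens a level.
; Each DrawHUD checks the Loading flag on the player's AlienHero_BP character.
; While it is set, it removes the hero's HUD widget and draws a loading material sized to the screen.
; In that same pass it opens the level picked by LevelIdx from the hero's Levels array.
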(event EventBeginPlay)

(event Collision|EventActorBeginOverlap
  (params (OtherActor :type Actor%20Object%20Reference)))

(event EventTick
  (params (DeltaSeconds :type Float%20%28single-precision%29)))

(event EventDrawHUD
  (params (SizeX :type Integer) (SizeY :type Integer))
  ;[1 1 1] Loading
  (Variables|Default|SetScreenDimensions (Math|Vector2D|MakeVector2D (Math|Conversions|ToFloat(Integer) SizeX) (Math|Conversions|ToFloat(Integer) SizeY)))
  (bind _asalien_hero_bp (Utilities|Casting|CastToAlienHero_BP (Game|GetPlayerCharacter 0)))
  (if (Variables|/Game/Dream/Blueprints/Gameplay/AlienHero_BP.AlienHero_BP_C|GetLoading _asalien_hero_bp)
    (Widget|RemovefromParent (Variables|/Game/Dream/Blueprints/Gameplay/AlienHero_BP.AlienHero_BP_C|Gethud_Widget _asalien_hero_bp))
    (Class|HUD|DrawMaterialSimple "/Game/Dream/Backgrounds/Textures/LoadingScreenMaterial.LoadingScreenMaterial" 0.0 0.0 (.x (Variables|Default|GetScreenDimensions)) (.y (Variables|Default|GetScreenDimensions)) 1.0 false)
    (Game|OpenLevel(byName) (Utilities|String|StringToName (Utilities|Array|Get(acopy) (Variables|/Game/Dream/Blueprints/Gameplay/AlienHero_BP.AlienHero_BP_C|GetLevels _asalien_hero_bp) (Variables|Default|GetLevel_Idx))))))

(fn ConstructionScript)