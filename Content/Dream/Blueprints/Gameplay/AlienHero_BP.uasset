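; AlienHero_BP is the 2D side-scroller player character, with movement, jump, crouch, touch jump and a HUD.
; A state variable picks flipbooks from arrays indexed by the character loaded from the MenuData save.
; Gated damage applies knockback and blinking until landing restores input, with key 1 triggering test damage.
; Death, triggered on landing or by a delayed Tick fallback, respawns a new hero at the checkpoint with carried-over stats or shows Game Over.
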(event Custom|DamageSystem
  (params (DamageIn :type Float%20%28single-precision%29))
  ;[1 1 1] Damage System
  (Utilities|FlowControl|Gate false :!label _label
    (:Exit
      (Utilities|FlowControl|Sequence
        (:then_0
          (goto _label Close))
        (:then_1
          (Variables|Default|SetIsHit true)
          (Input|DisableInput (Game|GetPlayerController 0))
          (bind _output_get (Variables|Default|SetCurrentHealth (- (Variables|Default|GetCurrentHealth) DamageIn)))
          (if (<= _output_get 0.0)
            (Variables|Default|SetState "NewEnumerator5")
            (Variables|Default|SetIsDead true)
            (Input|DisableInput (Game|GetPlayerController 0))
            (CallFunction|UpdateAnimation)
            (else
              (Variables|Default|SetState "NewEnumerator4")
              (Physics|AddForce (Variables|Character|GetCharacterMovement) (Math|Vector|MakeVector (* (Variables|Default|GetDirectionFacing) (Variables|Default|GetKnockbackForce)) 0.0 2e+06))
              (Utilities|Time|SetTimerbyFunctionName 0 "Blink" 0.1 true)
              (Utilities|FlowControl|Delay 2.5)
              (Utilities|Time|ClearTimerbyFunctionName 0 "Blink")
              (goto _label Open))))))))

(event Custom|UpdateAnimation
  (bind _character_ref (Variables|Default|GetCharacter_Ref))
  ;[1 1 1] Handle Animation
  (switch Utilities|FlowControl|Switch|SwitchonChar_States (Variables|Default|GetState)
    (:NewEnumerator0
      (Sprite|SetFlipbook (Variables|Default|GetSprite) (select (> (Math|Vector|VectorLength (Transformation|GetVelocity)) 0.0) (Utilities|Array|Get(acopy) (Variables|Default|Getfliparray_walk) _character_ref) (Utilities|Array|Get(acopy) (Variables|Default|Getfliparray_idle) _character_ref))))
    (:NewEnumerator2
      (Sprite|SetFlipbook (Variables|Default|GetSprite) (Utilities|Array|Get(acopy) (Variables|Default|Getfliparray_jump) (Variables|Default|GetCharacter_Ref))))
    (:NewEnumerator3
      (Sprite|SetFlipbook (Variables|Default|GetSprite) (Utilities|Array|Get(acopy) (Variables|Default|Getfliparray_crouch) (Variables|Default|GetCharacter_Ref))))
    (:NewEnumerator4
      (Sprite|SetFlipbook (Variables|Default|GetSprite) (Utilities|Array|Get(acopy) (Variables|Default|Getfliparray_hit) (Variables|Default|GetCharacter_Ref)) :!label _label))
    (:NewEnumerator5
      (goto _label))))

(event Custom|Death%20Bug
  (bind _sprite (Variables|Default|GetSprite))
  ;[1 1 1] Death
  ;;[1 1 1] If There Is A Death Bug
  (Collision|SetCollisionEnabled (Variables|Collision|GetCapsuleComponent) "NoCollision")
  (Class|SceneComponent|DetachfromParent (Variables|Camera|GetCameraBoom) true true)
  (bind (_direction _rotation_yaw _rotation_roll) (Timeline|Dead%20Timeline Play)
    (:Update
      (Transformation|SetWorldLocationAndRotation _sprite (Transformation|GetWorldLocation _sprite) (Math|Rotator|MakeRotator 15.0 _rotation_yaw _rotation_roll) false)
      (Utilities|FlowControl|Delay 2.5)
      (if (<= (Variables|Default|GetLives) 0)
        (CallFunction|GameOver)
        (else
          (Variables|Default|SetLives (- (Variables|Default|GetLives) 1))
          (Actor|DestroyActor)
          (CallFunction|SpawnPlayer "AlienHero_BP_C" (Variables|Default|GetLastCheckpoint) false)
          (bind _outactors (Actor|GetAllActorsOfClass "AlienHero_BP_C"))
          ;;[1 1 1] Set Info for New Actor
          (Variables|AlienHero_BP_C|SetCurrentHealth (Utilities|Array|Get(acopy) _outactors) 1.0)
          (Variables|AlienHero_BP_C|SetJewels (Utilities|Array|Get(acopy) _outactors) (Variables|Default|GetJewels))
          (Variables|AlienHero_BP_C|SetCharacter_Ref (Utilities|Array|Get(acopy) _outactors) (Variables|Default|GetCharacter_Ref))
          (bind _output_get (Variables|AlienHero_BP_C|SetLives (Utilities|Array|Get(acopy) _outactors) (Variables|Default|GetLives)))
          (if (<= _output_get 0)
            (CallFunction|GameOver)))))))

(event Custom|Blink
  (bind _sprite (Variables|Default|GetSprite))
  ;[1 1 1] Damage System
  ;;[1 1 1] Blinking
  (Development|SetHiddeninGame _sprite true false)
  (Utilities|FlowControl|Delay 0.1)
  (Development|SetHiddeninGame _sprite false false))

(event Custom|GameOver
  ;[1 1 1] Game Over Menu
  (Utilities|IsValid (Variables|Default|GetGameOverMenu_Ref)
    (:Is%20Valid
      _)
    (:Is%20Not%20Valid
      (bind _returnvalue (UserInterface|CreateWidget "/Game/Dream/Blueprints/Menus+HUDS/gameover_menu.gameover_menu_C" (Game|GetPlayerController 0)))
      (bind _output_get (Variables|Default|SetGameOverMenu_Ref _returnvalue))))
  (Input|SetInputModeUIOnly (Game|GetPlayerController 0) _output_get false)
  (UserInterface|Viewport|AddtoViewport (Variables|Default|GetGameOverMenu_Ref) 2))

(event Custom|Load%20Data
  ;[1 1 1] Load Data
  (bind _returnvalue (SaveGame|DoesSaveGameExist "MenuData"))
  (if _returnvalue
    (bind _returnvalue_2 (SaveGame|LoadGamefromSlot "MenuData"))
    (bind _asgame_data (Utilities|Casting|CastToGameData _returnvalue_2))
    (Variables|Default|SetCharacter_Ref (Variables|/Game/Dream/Save/GameData.GameData_C|GetCharacter_Select _asgame_data))
    (Variables|Default|SetVolume_Ref (Variables|/Game/Dream/Save/GameData.GameData_C|GetVolumeVal _asgame_data))))

(event EventOnLanded
  (params (Hit :type Hit%20Result%20Structure%20%28by%20ref%29))
  (bind _sprite (Variables|Default|GetSprite))
  (Utilities|FlowControl|Sequence
    (:then_0
      ;[1 1 1] Handle Landing
      (if (AI|Components|NavMovement|IsCrouching (Variables|Character|GetCharacterMovement))
        (if (Variables|Default|GetIsHit)
          (Variables|Default|SetState "NewEnumerator0" :!label _label)
          (CallFunction|UpdateAnimation)
          (Input|EnableInput (Game|GetPlayerController 0)))
        (elif (not (Variables|Default|GetIsDead))
          (if (Variables|Default|GetIsHit)
            (goto _label)
            (else
              (Variables|Default|SetState "NewEnumerator0")
              (CallFunction|UpdateAnimation))))))
    (:then_1
      ;[1 1 1] Death
      (if (Variables|Default|GetIsDead)
        (Variables|Default|SetDeath_Bug true)
        (Collision|SetCollisionEnabled (Variables|Collision|GetCapsuleComponent) "NoCollision")
        (Class|SceneComponent|DetachfromParent (Variables|Camera|GetCameraBoom) true true)
        (bind (_direction _rotation_yaw _rotation_roll) (Timeline|Dead%20Timeline Play)
          (:Update
            (Transformation|SetWorldLocationAndRotation _sprite (Transformation|GetWorldLocation _sprite) (Math|Rotator|MakeRotator 15.0 _rotation_yaw _rotation_roll) false)
            (Utilities|FlowControl|Delay 2.5)
            (if (<= (Variables|Default|GetLives) 0)
              (CallFunction|GameOver)
              (else
                (Variables|Default|SetLives (- (Variables|Default|GetLives) 1))
                (Actor|DestroyActor)
                (CallFunction|SpawnPlayer "AlienHero_BP_C" (Variables|Default|GetLastCheckpoint) false)
                (bind _outactors (Actor|GetAllActorsOfClass "AlienHero_BP_C"))
                ;;[1 1 1] Set Info for New Actor
                (Variables|AlienHero_BP_C|SetCurrentHealth (Utilities|Array|Get(acopy) _outactors) 1.0)
                (Variables|AlienHero_BP_C|SetJewels (Utilities|Array|Get(acopy) _outactors) (Variables|Default|GetJewels))
                (Variables|AlienHero_BP_C|SetCharacter_Ref (Utilities|Array|Get(acopy) _outactors) (Variables|Default|GetCharacter_Ref))
                (bind _output_get (Variables|AlienHero_BP_C|SetLives (Utilities|Array|Get(acopy) _outactors) (Variables|Default|GetLives)))
                (if (<= _output_get 0)
                  (CallFunction|GameOver))))))))))

(event EventBeginPlay
  ;[1 1 1] Initialize
  (CallFunction|LoadData)
  (Utilities|FlowControl|Sequence
    (:then_0
      (Class|ActorComponent|SetIsReplicated (Variables|Default|GetSprite) true))
    (:then_1
      (bind _returnvalue (UserInterface|CreateWidget "/Game/Dream/Blueprints/Menus+HUDS/screen_HUD.screen_HUD_C" (Game|GetPlayerController 0)))
      (bind _output_get (Variables|Default|Sethud_Widget _returnvalue))
      (UserInterface|Viewport|AddtoViewport _output_get 1)
      (Variables|Default|SetPlayerPawn (Game|Player|GetPlayerPawn 0)))))

(event EventTick
  (params (DeltaSeconds :type Float%20%28single-precision%29))
  ;[1 1 1] If There Is A Death Bug
  (if (Variables|Default|GetIsDead)
    (Utilities|FlowControl|Delay 3.0)
    (if (not (Variables|Default|GetDeath_Bug))
      (CallFunction|DeathBug))))

(event Input|ActionEvents|InputActionCrouch
  ;[1 1 1] Handle Crouch
  (:Pressed
    (Variables|Default|SetState "NewEnumerator3")
    (Character|Crouch)
    (CallFunction|UpdateAnimation))
  (:Released
    (Variables|Default|SetState "NewEnumerator0")
    (Character|UnCrouch)
    (CallFunction|UpdateAnimation)))

(event Input|ActionEvents|InputActionJump
  ;[1 1 1] Handle Jump
  (:Pressed
    (if (Character|CanJump)
      (Character|Jump)
      (Variables|Default|SetState "NewEnumerator2")))
  (:Released
    (Character|StopJumping)))

(event Input|AxisEvents|InputAxisMoveRight
  (params (AxisValue :type Float%20%28single-precision%29))
  (bind _sprite (Variables|Default|GetSprite))
  ;[1 1 1] Handle movement
  (CallFunction|UpdateAnimation)
  (if (> AxisValue 0.0)
    (Transformation|SetRelativeRotation _sprite "0,0.000000, 0" false)
    (Variables|Default|SetDirectionFacing -1)
    (Pawn|Input|AddMovementInput "1.000000, 0, 0" AxisValue false :!label _label)
    (elif (< AxisValue 0.0)
      (Transformation|SetRelativeRotation _sprite "0.000000,180.000000,0.000000" false)
      (Variables|Default|SetDirectionFacing 1)
      (goto _label))))

(event Input|KeyboardEvents|1
  ;[1 1 1] Damage System
  (:Pressed
    (CallFunction|DamageSystem 0.5)))

(event Input|TouchEvents|InputTouch
  (params (Location :type Vector) (FingerIndex :type ETouchIndex%20Enum))
  ;[1 1 1] Handle Jump
  (:Pressed
    (if (Character|CanJump)
      (Character|Jump)
      (Variables|Default|SetState "NewEnumerator2")))
  (:Released
    (Character|StopJumping)))

(fn ConstructionScript)

(fn SpawnPlayer
  (params (Class :type Actor%20Class%20Reference) (Transform :type Transform) (Random :type Boolean))
  (if (Math|Vector|NotEqual(Vector) (.Location (Math|Transform|BreakTransform Transform)) "0, 0,0.000000" 0.0001)
    (bind _returnvalue (Game|SpawnActorfromClass Class Transform false 0 0))
    (bind _aspawn (Utilities|Casting|CastToPawn _returnvalue))
    (bind _output_get (Variables|Default|SetPlayerPawn _aspawn))
    (else
      (bind _outactors (Actor|GetAllActorsOfClass "/Script/Engine.PlayerStart"))
      (if Random
        (Variables|Default|SetLastSpawn (Utilities|Array|Get(acopy) _outactors (Math|Random|RandomInteger (Utilities|Array|Length _outactors))))
        (else
          (bind _array_element (Utilities|Array|ForEachLoopwithBreak _outactors :!label _label)
            (:LoopBody
              (Variables|Default|SetLastSpawn _array_element)
              (goto _label Break))
            (:Completed
              _))))
      (bind _returnvalue_2 (Game|SpawnActorfromClass Class (Transformation|GetActorTransform (Variables|Default|GetLastSpawn)) false 0 0))
      (bind _aspawn_2 (Utilities|Casting|CastToPawn _returnvalue_2))
      (Variables|Default|SetPlayerPawn _aspawn_2)))
  (Pawn|Possess (Game|GetPlayerController 0) _output_get))

(fn GetPlayerLocation
  (return (Transformation|GetActorTransform)))

(fn GetCheckpoint
  (bind _lastcheckpoint (Variables|Default|GetLastCheckpoint))
  (return _lastcheckpoint (Math|Vector|NotEqual(Vector) (.Location (Math|Transform|BreakTransform _lastcheckpoint)) "0, 0, 0" 0.0001)))

(fn SetCheckpoint
  (params (Update :type Boolean))
  (bind _location (CallFunction|GetPlayerLocation))
  (Variables|Default|SetLastCheckpoint _location)
  (return (Math|Vector|NotEqual(Vector) (.Location (Math|Transform|BreakTransform (Variables|Default|GetLastCheckpoint))) "0, 0, 0" 0.0001)))