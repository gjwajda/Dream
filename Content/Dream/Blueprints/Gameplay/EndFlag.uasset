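; EndFlag is the level-ending flag that completes the game when the player's AlienHero_BP reaches it with exactly three jewels.
; Its sphere overlap plays a win sound at the hero's stored volume and switches the flag's flipbook to the blue animation.
; It then creates the End_Level1 widget if none exists, switches input to UI only and shows the screen.
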(event OnComponentBeginOverlap(Sphere)
  (params (OtherActor :type Actor%20Object%20Reference) (OtherComp :type Primitive%20Component%20Object%20Reference) (OtherBodyIndex :type Integer) (bFromSweep :type Boolean) (SweepResult :type Hit%20Result%20Structure%20%28by%20ref%29))
  ;[1 1 1] End Game
  (bind _asalien_hero_bp (Utilities|Casting|CastToAlienHero_BP OtherActor))
  (if (== (Variables|/Game/Dream/Blueprints/Gameplay/AlienHero_BP.AlienHero_BP_C|GetJewels _asalien_hero_bp) 3)
    (Audio|PlaySoundatLocation "/Game/Dream/Audio/win_Cue.win_Cue" (Transformation|GetActorLocation) (Variables|/Game/Dream/Blueprints/Gameplay/AlienHero_BP.AlienHero_BP_C|GetVolume_Ref _asalien_hero_bp))
    (Sprite|SetFlipbook (Variables|Default|GetFlag) "/Game/Dream/HUD/Items/flagBlue_animation.flagBlue_animation")
    (Utilities|IsValid (Variables|Default|GetGameEnd_ref)
      (:Is%20Valid
        _)
      (:Is%20Not%20Valid
        (bind _returnvalue (UserInterface|CreateWidget "/Game/Dream/Blueprints/Menus+HUDS/End_Level1.End_Level1_C" (Game|GetPlayerController 0)))
        (bind _output_get (Variables|Default|SetGameEnd_ref _returnvalue))))
    (Input|SetInputModeUIOnly (Game|GetPlayerController 0) _output_get false)
    (UserInterface|Viewport|AddtoViewport (Variables|Default|GetGameEnd_ref) 2)))

(event EventBeginPlay)

(event Collision|EventActorBeginOverlap
  (params (OtherActor :type Actor%20Object%20Reference)))

(event EventTick
  (params (DeltaSeconds :type Float%20%28single-precision%29)))

(fn ConstructionScript)