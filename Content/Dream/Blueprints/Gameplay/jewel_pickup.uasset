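; Jewel pickup actor that the AlienHero_BP player collects by touching it.
; A timeline started on BeginPlay drives the yaw and adds its Z value to the current height on each update.
; Sphere overlap by the hero increments its Jewels count, plays a coin sound scaled by the hero's VolumeRef, then destroys the actor.
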(event OnComponentBeginOverlap(Sphere)
  (params (OtherActor :type Actor%20Object%20Reference) (OtherComp :type Primitive%20Component%20Object%20Reference) (OtherBodyIndex :type Integer) (bFromSweep :type Boolean) (SweepResult :type Hit%20Result%20Structure%20%28by%20ref%29))
  ;[1 1 1] Collect
  (bind _asalien_hero_bp (Utilities|Casting|CastToAlienHero_BP OtherActor))
  (Variables|/Game/Dream/Blueprints/Gameplay/AlienHero_BP.AlienHero_BP_C|SetJewels _asalien_hero_bp (+ (Variables|/Game/Dream/Blueprints/Gameplay/AlienHero_BP.AlienHero_BP_C|GetJewels _asalien_hero_bp) 1))
  (Audio|PlaySoundatLocation "/Game/Dream/Audio/Coin_Cue.Coin_Cue" (Transformation|GetActorLocation) (* 2 (Variables|/Game/Dream/Blueprints/Gameplay/AlienHero_BP.AlienHero_BP_C|GetVolume_Ref _asalien_hero_bp)))
  (Actor|DestroyActor))

(event EventBeginPlay
  (bind _returnvalue (Transformation|GetActorLocation))
  ;[1 1 1] Rotate
  (bind (_direction _z_rotation _z_location) (Timeline|Jewel%20Rotation Play)
    (:Update
      (Transformation|SetActorLocationAndRotation (Math|Vector|MakeVector (.x _returnvalue) (.y _returnvalue) (+ _z_location (.z _returnvalue))) (Math|Rotator|MakeRotator 0.0 _z_rotation 0.0)))))

(event Collision|EventActorBeginOverlap
  (params (OtherActor :type Actor%20Object%20Reference)))

(event EventTick
  (params (DeltaSeconds :type Float%20%28single-precision%29)))

(fn ConstructionScript)